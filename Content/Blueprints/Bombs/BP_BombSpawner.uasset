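; Spawner that drops cluster, homing or laser bombs at random points inside its SpawningArea box.
; A looping timer, with its interval randomized once at BeginPlay, picks one type at random; homing bombs target player character 0.
; Each spawner function rolls stats from min/max ranges and derives some from others, such as laser speed divided by count.
; Cluster and homing bombs are configured and ignited through events, while lasers receive values at spawn.
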(event Custom|Event_SpawnOverTime
  (switch int (Math|Random|RandomIntegerinRange 0 2)
    (:Default
      (CallFunction|BombTypeClusterSpawner :!label _label))
    (:0
      (goto _label))
    (:1
      (CallFunction|BombTypeHomingSpawner))
    (:2
      (CallFunction|BombTypeLaserSpawner))))

(event EventBeginPlay
  (Utilities|Time|SetTimerbyEvent (delegate Custom|Event_SpawnOverTime) (Math|Random|RandomFloatinRange 0.5 1.5) true)
  (Variables|Default|SetHomingTarget (Game|GetPlayerCharacter 0)))

(fn ConstructionScript)

(fn BombTypeClusterSpawner
  (bind _spawningarea (Variables|Default|GetSpawningArea))
  (bind _minclustercount (Variables|Default|GetMinClusterCount))
  (bind _maxclustercount (Variables|Default|GetMaxClusterCount))
  (bind _returnvalue (Math|Random|RandomIntegerinRange _minclustercount _maxclustercount))
  (bind _returnvalue_2 (Game|SpawnActorfromClass (Variables|Default|GetBombTypeCluster) (Math|Transform|MakeTransform (Math|Random|RandomPointinBoundingBox (Transformation|GetWorldLocation _spawningarea) (Variables|/Script/Engine.BoxComponent|GetBoxExtent _spawningarea)) "-90.000000,0.000000,0.000000") "Undefined" "MultiplyWithRoot" 0 0))
  (bind _asbp_bomb_type_cluster (Utilities|Casting|CastToBP_BombTypeCluster _returnvalue_2))
  (Default|EventSetAttributes _asbp_bomb_type_cluster (Math|Random|RandomFloatinRange (Variables|Default|GetMinDelay) (Variables|Default|GetMaxDelay)) (Math|Random|RandomFloatinRange (Variables|Default|GetMinRadius) (Variables|Default|GetMaxRadius)) _returnvalue (Math|Random|RandomIntegerinRange (Math|Integer|Clamp(Integer) (- _returnvalue 4) 2 _maxclustercount) (Math|Integer|Clamp(Integer) _returnvalue 2 _maxclustercount)))
  (Default|EventIgnite _asbp_bomb_type_cluster))

(fn BombTypeHomingSpawner
  (bind _spawningarea (Variables|Default|GetSpawningArea))
  (bind _mindelay (Variables|Default|GetMinDelay))
  (bind _maxdelay (Variables|Default|GetMaxDelay))
  (bind _minhomingspeed (Variables|Default|GetMinHomingSpeed))
  (bind _maxhomingspeed (Variables|Default|GetMaxHomingSpeed))
  (bind _returnvalue (Math|Random|RandomFloatinRange _minhomingspeed _maxhomingspeed))
  (bind _returnvalue_2 (Math|Random|RandomFloatinRange _mindelay _maxdelay))
  (bind _returnvalue_3 (/ _returnvalue _returnvalue_2))
  ;[0.84 0.15 0.15 0.5] Spawns the missile
  (bind _returnvalue_4 (Game|SpawnActorfromClass "/Game/Blueprints/Bombs/BP_BombTypeHoming.BP_BombTypeHoming_C" (Math|Transform|MakeTransform (Math|Random|RandomPointinBoundingBox (Transformation|GetWorldLocation _spawningarea) (Variables|/Script/Engine.BoxComponent|GetBoxExtent _spawningarea)) "-90.000000,0.000000,0.000000") "Undefined" "MultiplyWithRoot" 0 (Actor|GetComponentbyClass (Variables|Default|GetHomingTarget) "/Script/Engine.SceneComponent") 0))
  (bind _asbp_bomb_type_homing (Utilities|Casting|CastToBP_BombTypeHoming _returnvalue_4))
  (Default|EventSetAttributes _asbp_bomb_type_homing (* _returnvalue_2 3.0) (/ (Math|Random|RandomFloatinRange (Variables|Default|GetMinRadius) (Variables|Default|GetMaxRadius)) 2.0) _returnvalue_3 (/ (- _maxhomingspeed _returnvalue_3) 3.0))
  (Default|EventIgnite _asbp_bomb_type_homing))

(fn BombTypeLaserSpawner
  (bind _minlasercount (Variables|Default|GetMinLaserCount))
  (bind _maxlasercount (Variables|Default|GetMaxLaserCount))
  (bind _spawningarea (Variables|Default|GetSpawningArea))
  (bind _returnvalue (Math|Random|RandomIntegerinRange _minlasercount _maxlasercount))
  ;[0.84 0.15 0.15 0.5] Spawns the missile
  (Game|SpawnActorfromClass "/Game/Blueprints/Bombs/BP_BombTypeLaser.BP_BombTypeLaser_C" (Math|Transform|MakeTransform (Math|Random|RandomPointinBoundingBox (Transformation|GetWorldLocation _spawningarea) (Variables|/Script/Engine.BoxComponent|GetBoxExtent _spawningarea)) "0.000000,0.000000,0.000000") "Undefined" "MultiplyWithRoot" 0 (Math|Random|RandomFloatinRange (Variables|Default|GetMinDelay) (Variables|Default|GetMaxDelay)) (Math|Random|RandomFloatinRange (Variables|Default|GetMinRadius) (Variables|Default|GetMaxRadius)) _returnvalue (/ (Math|Random|RandomFloatinRange (Variables|Default|GetMinLaserSpeed) (Variables|Default|GetMaxLaserSpeed)) _returnvalue) (Math|Random|RandomFloatinRange (Variables|Default|GetMinLaserDuration) (Variables|Default|GetMaxLaserDuration)) 0))