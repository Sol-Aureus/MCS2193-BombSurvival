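; BP_BombTypeLaser is a timed bomb that explodes and leaves spinning lasers behind.
; After a delay from BeginPlay, a sphere trace kills the player once and destroys other actors tagged Killable.
; It then spawns BP_Laser actors at its centre, yawed evenly across 180 degrees, passing them lifetime and spin speed, and destroys itself.
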(event EventBeginPlay
  (bind _box (Variables|Default|GetBox))
  (bind _returnvalue (Transformation|GetWorldLocation _box))
  ;[0.8174 0.3652 0.3391 0.5] Explode
  (Utilities|FlowControl|Delay (Variables|Default|GetDetonationDelay))
  (Variables|Default|SetHitPlayer false)
  (bind _outhits (Collision|MultiSphereTraceForObjects _returnvalue _returnvalue (Variables|Default|GetExplosionRadius) (Utilities|Array|MakeArray "ObjectTypeQuery3" "ObjectTypeQuery1") false 0 "ForOneFrame"))
  ;[0.15 0.15 0.9478 0.5] Check for targets
  (for _array_element _outhits
    (CallFunction|CheckTargets (.HitActor (Collision|BreakHitResult _array_element))))
  ;[0.15 0.9043 0.15 0.5] Spawn bomblets
  (CallFunction|SpawnLasers (Variables|Default|GetLaserCount) (Variables|Default|GetLaserDuration) (Variables|Default|GetLaserSpeed))
  (Actor|DestroyActor))

(fn ConstructionScript)

(fn CheckTargets
  (params (Object :type Actor%20Object%20Reference))
  (if (Actor|ActorHasTag Object "Player")
    ;[1 0.15 0.15 0.5] If the player is hit, call their kill function
    (if (not (Variables|Default|GetHitPlayer))
      (Variables|Default|SetHitPlayer true)
      (bind _asbp_player_character (Utilities|Casting|CastToBP_PlayerCharacter Object))
      (Default|EventKill _asbp_player_character))
    (else
      ;[0.15 0.15 1 0.5] Otherwise just delete it
      (if (Actor|ActorHasTag Object "Killable")
        (Actor|DestroyActor Object)))))

(fn SpawnLasers
  (params (Count :type Integer) (Duration :type Float%20%28double-precision%29) (Speed :type Float%20%28double-precision%29))
  (bind _box (Variables|Default|GetBox))
  (bind _returnvalue (Transformation|GetWorldLocation _box))
  ;[1 0.1092 0 0.5] Change this to spawn lasers instead
  (if (> Count 0)
    (for _index (range 1 Count)
      ;[0.15 0.913 1 0.5] Spawning the bomblets
      (bind _outhit (Collision|LineTraceForObjects _returnvalue (+ _returnvalue (Math|Vector|RotateVector (Math|Vector|GetForwardVector "0, 0, 0") (Math|Rotator|MakeRotator 0.0 0.0 (* _index (/ 1.8e+02 (Math|Conversions|ToFloat(Integer) Count)))))) (Utilities|Array|MakeArray "ObjectTypeQuery1") false 0 "ForOneFrame"))
      (Game|SpawnActorfromClass "/Game/Blueprints/Bombs/BP_Laser.BP_Laser_C" (Math|Transform|MakeTransform (.TraceEnd (Collision|BreakHitResult _outhit)) (Math|Rotator|MakeRotator 0.0 0.0 (* _index (/ 1.8e+02 (Math|Conversions|ToFloat(Integer) Count))))) "Undefined" "MultiplyWithRoot" 0 Duration Speed 0))))