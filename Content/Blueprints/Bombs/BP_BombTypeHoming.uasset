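; BP_BombTypeHoming is a homing missile bomb that explodes on collider overlap or when its ignited countdown ends.
; A setup event configures delay, blast radius, speed and homing on its ProjectileMovement, while Tick turns the collider along its velocity.
; The explosion sphere-traces Pawn and WorldStatic objects, kills the player once, destroys non-player actors tagged Killable, then destroys itself.
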(event OnComponentBeginOverlap(Collider)
  (params (OverlappedComponent :type Primitive%20Component%20Object%20Reference) (OtherActor :type Actor%20Object%20Reference) (OtherComp :type Primitive%20Component%20Object%20Reference) (OtherBodyIndex :type Integer) (bFromSweep :type Boolean) (SweepResult :type Hit%20Result%20Structure%20%28by%20ref%29))
  (bind _collider (Variables|Default|GetCollider))
  (bind _returnvalue (Transformation|GetWorldLocation _collider))
  ;[0.8174 0.3652 0.3391 0.5] Explode
  (Variables|Default|SetHitPlayer false)
  (bind _outhits (Collision|MultiSphereTraceForObjects _returnvalue _returnvalue (Variables|Default|GetExplosionRadius) (Utilities|Array|MakeArray "ObjectTypeQuery3" "ObjectTypeQuery1") false 0 "ForOneFrame"))
  ;[0.15 0.15 0.9478 0.5] Check for targets
  (for _array_element _outhits
    (CallFunction|CheckTargets (.HitActor (Collision|BreakHitResult _array_element))))
  (Actor|DestroyActor))

(event Custom|Event_SetAttributes
  (params (Delay :type Float%20%28double-precision%29) (Radius :type Float%20%28double-precision%29) (MaxSpeed :type Float%20%28double-precision%29) (HomingAcceleration :type Float%20%28double-precision%29))
  (bind _projectilemovement (Variables|Default|GetProjectileMovement))
  ;[1 0.6783 0.15 0.5] Sets the attributes upon being summoned
  (Utilities|FlowControl|Sequence
    (:then_0
      (Variables|Default|SetDetonationDelay Delay))
    (:then_1
      (Variables|Default|SetExplosionRadius Radius))
    (:then_2
      (Variables|/Script/Engine.ProjectileMovementComponent|SetMaxSpeed _projectilemovement MaxSpeed))
    (:then_3
      (Variables|/Script/Engine.ProjectileMovementComponent|SetHomingAccelerationMagnitude _projectilemovement HomingAcceleration))
    (:then_4
      (Variables|/Script/Engine.ProjectileMovementComponent|SetHomingTargetComponent _projectilemovement (Variables|Default|GetHoming%20Target%20Component)))))

(event Custom|Event_Ignite
  (bind _collider (Variables|Default|GetCollider))
  (bind _returnvalue (Transformation|GetWorldLocation _collider))
  ;[1 0.15 0.15 0.5] Start the count down
  (Utilities|FlowControl|Delay (Variables|Default|GetDetonationDelay))
  ;[0.8174 0.3652 0.3391 0.5] Explode
  (Variables|Default|SetHitPlayer false)
  (bind _outhits (Collision|MultiSphereTraceForObjects _returnvalue _returnvalue (Variables|Default|GetExplosionRadius) (Utilities|Array|MakeArray "ObjectTypeQuery3" "ObjectTypeQuery1") false 0 "ForOneFrame"))
  ;[0.15 0.15 0.9478 0.5] Check for targets
  (for _array_element _outhits
    (CallFunction|CheckTargets (.HitActor (Collision|BreakHitResult _array_element))))
  (Actor|DestroyActor))

(event EventTick
  (params (DeltaSeconds :type Float%20%28single-precision%29))
  (bind _returnvalue (Transformation|GetActorLocation))
  ;[0.527 0.9235 0.8748 0.5] Rotates the missile towards it's movement direction
  (Transformation|SetWorldRotation (Variables|Default|GetCollider) (Math|Rotator|FindLookatRotation _returnvalue (+ _returnvalue (Variables|/Script/Engine.MovementComponent|GetVelocity (Variables|Default|GetProjectileMovement)))) false false))

(fn ConstructionScript)

(fn CheckTargets
  (params (Object :type Actor%20Object%20Reference))
  (if (Actor|ActorHasTag Object "Player")
    ;[1 0.15 0.15 0.5] If the player is hit, call their kill function
    (if (not (Variables|Default|GetHitPlayer))
      (Variables|Default|SetHitPlayer true)
      (bind _asbp_player_character (Utilities|Casting|CastToBP_PlayerCharacter Object))
      (Default|EventKill _asbp_player_character))
    (else
      ;[0.15 0.15 1 0.5] Otherwise just delete it
      (if (Actor|ActorHasTag Object "Killable")
        (Actor|DestroyActor Object)))))