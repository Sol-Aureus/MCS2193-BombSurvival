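; Cluster bomb actor that explodes after a delay, then spawns smaller-count generations of itself.
; The blast sphere-traces for pawns and static objects, killing the player once and destroying actors tagged Killable.
; It recursively spawns bomblets in a pitched radial ring with randomized delay and radius, reducing their count each generation.
; Bomblets spawn at each line trace's end point rather than its impact point.
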(event EventBeginPlay
  (bind _collider (Variables|Default|GetCollider))
  (bind _returnvalue (Transformation|GetWorldLocation _collider))
  ;[1 0.15 0.15 0.5] Start the count down
  (Utilities|FlowControl|Delay (Variables|Default|GetDetonationDelay))
  ;[0.8174 0.3652 0.3391 0.5] Explode
  (Variables|Default|SetHitPlayer false)
  (bind _outhits (Collision|MultiSphereTraceForObjects _returnvalue _returnvalue (Variables|Default|GetExplosionRadius) (Utilities|Array|MakeArray "ObjectTypeQuery3" "ObjectTypeQuery1") false 0 "ForOneFrame"))
  ;[0.15 0.15 0.9478 0.5] Check for targets
  (for _array_element _outhits
    (CallFunction|CheckTargets (.HitActor (Collision|BreakHitResult _array_element))))
  ;[0.15 0.9043 0.15 0.5] Spawn bomblets
  (CallFunction|SpawnBomblet (Variables|Default|GetBombletCount) (Variables|Default|GetDetonationDelay) (Variables|Default|GetExplosionRadius) (Variables|Default|GetBombletDistance) (Variables|Default|GetBombletSubtraction))
  (Actor|DestroyActor))

(fn ConstructionScript)

(fn CheckTargets
  (params (Object :type Actor%20Object%20Reference))
  (if (Actor|ActorHasTag Object "Player")
    ;[1 0.15 0.15 0.5] If the player is hit, call their kill function
    (if (not (Variables|Default|GetHitPlayer))
      (Variables|Default|SetHitPlayer true)
      (bind _asbp_player_character (Utilities|Casting|CastToBP_PlayerCharacter Object))
      (Default|EventKill _asbp_player_character))
    (else
      ;[0.15 0.15 1 0.5] Otherwise just delete it
      (if (Actor|ActorHasTag Object "Killable")
        (Actor|DestroyActor Object)))))

(fn SpawnBomblet
  (params (Count :type Integer) (Delay :type Float%20%28double-precision%29) (Radius :type Float%20%28double-precision%29) (Distance :type Float%20%28double-precision%29) (Subtraction :type Integer))
  (bind _collider (Variables|Default|GetCollider))
  (bind _bombletpitch (LocalVariables|GetBombletPitch))
  (bind _returnvalue (Transformation|GetWorldLocation _collider))
  ;[1 0.9739 0.3565 0.5] The math to spawn the bomblets radially
  (if (> Count 0)
    (for _index (range 1 Count)
      ;[0.15 0.913 1 0.5] Spawning the bomblets
      (bind _outhit (Collision|LineTraceForObjects _returnvalue (+ _returnvalue (* (Math|Vector|RotateVector (Math|Vector|GetForwardVector "0, 0, 0") (Math|Rotator|MakeRotator 0.0 _bombletpitch (* _index (/ 3.6e+02 (Math|Conversions|ToFloat(Integer) Count))))) Distance)) (Utilities|Array|MakeArray "ObjectTypeQuery1") false 0 "ForOneFrame"))
      (Game|SpawnActorfromClass "BP_BombTypeCluster_C" (Math|Transform|MakeTransform (.TraceEnd (Collision|BreakHitResult _outhit)) (Math|Rotator|MakeRotator 0.0 _bombletpitch (* _index (/ 3.6e+02 (Math|Conversions|ToFloat(Integer) Count))))) "Undefined" "MultiplyWithRoot" 0 (Math|Random|RandomFloatinRange (* Delay 0.9) (* Delay 1.1)) (Math|Random|RandomFloatinRange (* Radius 0.9) (* Radius 1.1)) (- Count Subtraction) Subtraction 0))))